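; BP_AudioVisualizer is an actor that displays a row of eight cubes as a bar-style spectrum visualizer for its Audio component.
; The construction script collects the cubes into an array and spaces them evenly along local Y.
; Each Tick reads cooked FFT data at eight fixed frequencies and interpolates each cube's Z scale toward its band's scaled magnitude, smoothing the motion.
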(event EventBeginPlay)

(event Collision|EventActorBeginOverlap
  (params (OtherActor :type Actor%20Object%20Reference)))

(event EventTick
  (params (DeltaSeconds :type Float%20%28single-precision%29))
  (bind _outsoundwavespectraldata (Class|AudioComponent|GetCookedFFTData (Variables|Default|GetAudio) (Utilities|Array|MakeArray 2e+02 4e+02 6e+02 8e+02 1e+03 2e+03 4e+03 8e+03)))
  (for (_array_element _array_index) _outsoundwavespectraldata
    (Transformation|SetRelativeScale3D (Utilities|Array|Get(acopy) (Variables|Default|GetCubes) _array_index) (Math|Interpolation|VInterpTo (Transformation|GetWorldScale (Utilities|Array|Get(acopy) (Variables|Default|GetCubes) _array_index)) (Math|Vector|MakeVector 1.0 1.0 (* (.Magnitude (Utilities|Struct|BreakSoundWaveSpectralData _array_element)) 0.2)) (Utilities|Time|GetWorldDeltaSeconds) 2.0))))

(fn ConstructionScript
  (bind _output_get (Variables|Default|SetCubes (Utilities|Array|MakeArray (Variables|Default|GetCube1) (Variables|Default|GetCube2) (Variables|Default|GetCube3) (Variables|Default|GetCube4) (Variables|Default|GetCube5) (Variables|Default|GetCube6) (Variables|Default|GetCube7) (Variables|Default|GetCube))))
  (for (_array_element _array_index) _output_get
    (Transformation|AddLocalOffset _array_element (Math|Vector|MakeVector 0.0 (* _array_index 1.2e+02) 0.0) false false)))